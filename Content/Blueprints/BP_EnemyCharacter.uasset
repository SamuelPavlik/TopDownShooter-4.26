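; Enemy character that matches walk speed to its animation and can spawn an explosion effect through DestroyEnemyEffect.
; While moving, Tick sets MaxWalkSpeed from the frame-to-frame change in left-foot-to-root distance along the facing direction, scaled by a fixed, frame-rate-dependent factor.
; StartMoving and StopMoving toggle this only when not falling, with stop zeroing speed.
; Construction tints a dynamic body material; debug speed prints remain.
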(event Custom|StopMoving
  (if (not (AI|Components|NavMovement|IsFalling (Variables|Character|GetCharacterMovement)))
    (Variables|/Script/Engine.CharacterMovementComponent|SetMaxWalkSpeed (Variables|Character|GetCharacterMovement) 0.0)
    (Variables|Default|SetIsMoving false)))

(event Custom|StartMoving
  (if (not (AI|Components|NavMovement|IsFalling (Variables|Character|GetCharacterMovement)))
    (Variables|Default|SetIsMoving true)))

(event EventBeginPlay)

(event Collision|EventActorBeginOverlap
  (params (OtherActor :type Actor%20Object%20Reference)))

(event EventTick
  (params (DeltaSeconds :type Float%20%28single-precision%29))
  (if (Variables|Default|GetIsMoving)
    (CallFunction|Move))
  (Variables|Default|SetLastRootToFoot (CallFunction|CalcRoottoFootProj)))

(event EventDestroyEnemyEffect
  (Game|SpawnActorfromClass "/Game/Blueprints/BP_Explosion.BP_Explosion_C" (Math|Transform|MakeTransform (Transformation|GetActorLocation) (Transformation|GetActorRotation) "1,1,1") "Undefined" 0 0))

(fn ConstructionScript
  (bind _returnvalue (Rendering|Material|CreateDynamicMaterialInstance (Variables|Character|GetMesh) 0 0 "None" :!class /Script/Engine.PrimitiveComponent))
  (bind _output_get (Variables|Default|SetDynaMat _returnvalue))
  (Rendering|Material|SetVectorParameterValue _output_get "BodyColor" (Variables|Default|GetColor) :!class /Script/Engine.MaterialInstanceDynamic))

(fn GetLegVelocity
  (bind _mesh (Variables|Character|GetMesh))
  (bind _charactermovement (Variables|Character|GetCharacterMovement))
  (bind _velocity (Variables|/Script/Engine.MovementComponent|GetVelocity _charactermovement))
  (bind _returnvalue (Math|Vector|Normalize _velocity))
  (return (* _returnvalue (Math|Vector|DotProduct _returnvalue (- (Transformation|GetSocketLocation _mesh "LeftFootSocket") (Transformation|GetSocketLocation _mesh "RootSocket"))))))

(fn Move
  (bind _output_get (Variables|/Script/Engine.CharacterMovementComponent|SetMaxWalkSpeed (Variables|Character|GetCharacterMovement) (* (- (CallFunction|CalcRoottoFootProj) (Variables|Default|GetLastRootToFoot)) -7e+01)))
  (Development|PrintString (Utilities|String|Append "Speed: " (Utilities|String|ToString(Float) _output_get)) true true "(R=0.000000,G=0.660000,B=1.000000,A=1.000000)" 1e+02)
  (Development|PrintString (Utilities|String|Append "Veloc: " (Utilities|String|ToString(Float) (Math|Vector|VectorLength (Variables|/Script/Engine.MovementComponent|GetVelocity (Variables|Character|GetCharacterMovement))))) true true "(R=0.000000,G=0.660000,B=1.000000,A=1.000000)" 1e+02))

(fn CalcRoottoFootProj
  (return (Math|Vector|DotProduct (Math|Vector|GetForwardVector (Class|CharacterMovementComponent|GetLastUpdateRotation (Variables|Character|GetCharacterMovement))) (- (Transformation|GetSocketLocation (Variables|Character|GetMesh) "LeftFootSocket") (Transformation|GetSocketLocation (Variables|Character|GetMesh) "RootSocket")))))