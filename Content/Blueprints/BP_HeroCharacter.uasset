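; BP_HeroCharacter is the player's hero character, carrying a weapon and owning the on-screen HUD.
; On BeginPlay it spawns BP_Weapon onto the mesh's GunSocket, has player controller 0 possess it and creates WBP_HUD, which is removed on destruction.
; ReloadEffect plays a reload montage and laser sound, holding IsReloading true until the montage completes.
; NoClipsEffect plays an out-of-clips montage.
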(event EventBeginPlay
  (bind _mesh (Variables|Character|GetMesh))
  (|CallParentFunction)
  (Utilities|FlowControl|Sequence
    (:then_0
      (bind _returnvalue (Game|SpawnActorfromClass "/Game/Blueprints/BP_Weapon.BP_Weapon_C" (Transformation|GetWorldTransform _mesh) "Undefined" 0 0))
      (bind _output_get (Variables|Default|SetWeapon _returnvalue))
      (Transformation|AttachComponentToComponent _output_get _mesh "GunSocket" "SnapToTarget" "KeepRelative" "KeepRelative" true))
    (:then_1
      (Pawn|Possess (Game|GetPlayerController 0) self)
      (bind _returnvalue_2 (UserInterface|CreateWidget "/Game/UI/WBP_HUD.WBP_HUD_C"))
      (UserInterface|Viewport|AddtoViewport _returnvalue_2 0)
      (Variables|Default|SetHUD _returnvalue_2))))

(event EventDestroyed
  (|CallParentFunction)
  (Widget|RemovefromParent (Variables|Default|GetHUD)))

(event EventReloadEffect
  (Variables|Default|SetbIsReloading true)
  (Animation|Montage|PlayMontage (Variables|Character|GetMesh) "/Game/AnimationAssets/AM_Reload_Rifle_Hip.AM_Reload_Rifle_Hip"
    (:then
      (Audio|PlaySoundatLocation "/Game/Audio/LaserReload.LaserReload" (.location (Transformation|GetActorTransform)) "0, 0, 0" 1.0 1.0 0.0 0 0 0))
    (:OnCompleted
      (Variables|Default|SetbIsReloading false))))

(event EventNoClipsEffect
  (Animation|Montage|PlayMontage (Variables|Character|GetMesh) "/Game/AnimationAssets/AM_NoClips.AM_NoClips"))

(fn ConstructionScript)