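; Character Blueprint for the menu hero, an armed character that can play a reload effect.
; On BeginPlay it spawns a BP_Weapon with an effectively bottomless clip, attaches it to the mesh's GunSocket, and stores all Brush actors in ActorsToIgnore.
; ReloadEffect plays the rifle hip reload montage with a laser reload sound, holding IsReloading true until the montage completes.
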(event EventBeginPlay
  (bind _mesh (Variables|Character|GetMesh))
  (Utilities|FlowControl|Sequence
    (:then_0
      (bind _returnvalue (Game|SpawnActorfromClass "/Game/Blueprints/BP_Weapon.BP_Weapon_C" (Transformation|GetWorldTransform _mesh) "Undefined" 0 0))
      (bind _output_get (Variables|Default|SetWeapon _returnvalue))
      (Variables|/Script/TopDownShooter.Weapon|SetCurrentClip _output_get 100000)
      (Transformation|AttachComponentToComponent _output_get _mesh "GunSocket" "SnapToTarget" "KeepRelative" "KeepRelative" true))
    (:then_1
      (bind _outactors (Actor|GetAllActorsOfClass "/Script/Engine.Brush"))
      (Variables|Default|SetActorsToIgnore _outactors))))

(event Collision|EventActorBeginOverlap
  (params (OtherActor :type Actor%20Object%20Reference)))

(event EventTick
  (params (DeltaSeconds :type Float%20%28single-precision%29)))

(event EventReloadEffect
  (Variables|Default|SetbIsReloading true)
  (Animation|Montage|PlayMontage (Variables|Character|GetMesh) "/Game/AnimationAssets/AM_Reload_Rifle_Hip.AM_Reload_Rifle_Hip"
    (:then
      (Audio|PlaySoundatLocation "/Game/Audio/LaserReload.LaserReload" (.location (Transformation|GetActorTransform)) "0, 0, 0" 1.0 1.0 0.0 0 0 0))
    (:OnCompleted
      (Variables|Default|SetbIsReloading false))))

(fn ConstructionScript)